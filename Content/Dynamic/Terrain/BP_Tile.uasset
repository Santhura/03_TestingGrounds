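; Terrain tile for an infinite terrain game that fills itself with randomly placed props and, unless the game mode flags a rest tile, enemy AI.
; Its barrier starts solid red; the player entering LockingVolume turns it green, disables its collision and calls TileConquered, and leaving relocks it.
; Player overlap with DestroyVolume asks the game mode to spawn the next tile, then destroys this tile and its props.
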(event `self.LockingVolume.OnComponentBeginOverlap`
  (params (OverlappedComponent :type "PrimitiveComponent Object Reference") (OtherActor :type "Actor Object Reference") (OtherComp :type "PrimitiveComponent Object Reference") (OtherBodyIndex :type Integer) (bFromSweep :type Boolean) (SweepResult :type "HitResult Structure (by ref)"))
  (`self.IsPlayerActor` OtherActor)
  (`|ExecutionSequence`
    (:`then_0`
      (`self.Unlock`))
    (:`then_1`
      (`self.TileConquered`))))

(event `self.LockingVolume.OnComponentEndOverlap`
  (params (OverlappedComponent :type "PrimitiveComponent Object Reference") (OtherActor :type "Actor Object Reference") (OtherComp :type "PrimitiveComponent Object Reference") (OtherBodyIndex :type Integer))
  (`self.IsPlayerActor` OtherActor)
  (`self.Lock`))

(event `self.Destroy Volume.OnComponentBeginOverlap`
  (params (OverlappedComponent :type "PrimitiveComponent Object Reference") (OtherActor :type "Actor Object Reference") (OtherComp :type "PrimitiveComponent Object Reference") (OtherBodyIndex :type Integer) (bFromSweep :type Boolean) (SweepResult :type "HitResult Structure (by ref)"))
  (`self.IsPlayerActor` OtherActor)
  (`self.SpawnNextTile`)
  (`self.DestroyProps`)
  (`self.K2_DestroyActor`))

(event `self.ReceiveBeginPlay`
  (`self.Lock`)
  (`self.SpawnPropsAndAI`))

(fn `GetAttachLocation`
  (returns (`Attach Transform` :type "Transform Structure"))
  (return (`SceneComponent.K2_GetComponentToWorld` (`self.Arrow`))))

(fn `Lock`
  (`PrimitiveComponent.SetCollisionEnabled` (`self.Barrier`) "QueryAndPhysics")
  (`PrimitiveComponent.SetMaterial` (`self.Barrier`) 0 "/Game/Dynamic/Terrain/MI_Barrier_Red.MI_Barrier_Red"))

(fn `SpawnNextTile`
  (bind _asinfinite_terrain_game_mode (cast `/Game/Dynamic/InfiniteTerrainGameMode` (`GameplayStatics.GetGameMode`)))
  (`/Game/Dynamic/InfiniteTerrainGameMode.SpawnTile` _asinfinite_terrain_game_mode))

(fn `SpawnPropsAndAI`
  (`self.PlaceActors` "/Game/Dynamic/Terrain/Props/BP_Container.BP_Container_C" (make `ActorProperties` 1 3 400.0))
  (`self.PlaceActors` "/Game/Dynamic/Terrain/Props/BP_Box.BP_Box_C" (make `ActorProperties` 2 4 100.0))
  (`self.PlaceActors` "/Game/Dynamic/Terrain/Props/BP_Canister.BP_Canister_C" (make `ActorProperties` 1 7 50.0))
  (`self.PlaceActors` "/Game/Dynamic/Terrain/Props/BP_Rock01.BP_Rock01_C" (make `ActorProperties` 2 4 150.0 0.8 5.0))
  (`self.PlaceActors` "/Game/Dynamic/Terrain/Props/BP_Rock05.BP_Rock05_C" (make `ActorProperties` 2 4 250.0 1.0 5.0))
  (`self.PlaceActors` "/Game/Dynamic/Terrain/Props/BP_Rock17.BP_Rock17_C" (make `ActorProperties` 2 4 250.0 1.0 5.0))
  (`self.PlaceActors` "/Game/Dynamic/Terrain/Props/BP_Sandbags.BP_Sandbags_C" (make `ActorProperties` 1 2 250.0))
  (bind _asinfinite_terrain_game_mode (cast `InfiniteTerrainGameMode` (`GameplayStatics.GetGameMode`)))
  (bind _returnvalue (`InfiniteTerrainGameMode.RestTile` _asinfinite_terrain_game_mode))
  (if (not _returnvalue)
    (`self.PlaceAIPawns` "/Game/Dynamic/Character/Behaviour/BP_Character.BP_Character_C" (make `ActorProperties` (`self.MinEnemies`) (`self.MaxEnemies`) 100.0))))

(fn `Unlock`
  (`PrimitiveComponent.SetCollisionEnabled` (`self.Barrier`) "NoCollision")
  (`PrimitiveComponent.SetMaterial` (`self.Barrier`) 0 "/Game/Dynamic/Terrain/MI_Barrier_Green.MI_Barrier_Green"))

(fn `UserConstructionScript`)